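; Teleporter beam actor that sends the actor overlapping its Beam component to a destination marked by an Arrow, placed from TeleportLocation in the construction script.
; Any overlap enables player input on the actor, and end overlap disables it.
; Pressing B moves the last overlapping actor's root to the Arrow's location and rotation.
; For the player character, it also aligns control rotation and zeroes velocity.
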(event OnComponentBeginOverlap(beam)
  (params (OverlappedComponent :type Primitive%20Component%20Object%20Reference) (OtherActor :type Actor%20Object%20Reference) (OtherComp :type Primitive%20Component%20Object%20Reference) (OtherBodyIndex :type Integer) (bFromSweep :type Boolean) (SweepResult :type Hit%20Result%20Structure%20%28by%20ref%29))
  (Input|EnableInput (Game|GetPlayerController 0)))

(event OnComponentEndOverlap(beam)
  (params (OverlappedComponent :type Primitive%20Component%20Object%20Reference) (OtherActor :type Actor%20Object%20Reference) (OtherComp :type Primitive%20Component%20Object%20Reference) (OtherBodyIndex :type Integer))
  (Input|DisableInput (Game|GetPlayerController 0)))

(event Input|KeyboardEvents|B
  (params (Key :type Key%20Structure :default "None"))
  (bind _returnvalue (Game|GetPlayerCharacter 0))
  (bind _arrow (Variables|Default|GetArrow))
  (bind _returnvalue_2 (Transformation|GetWorldTransform _arrow))
  (:Pressed
    (Transformation|SetWorldTransform (Variables|/Script/Engine.Actor|GetRootComponent (stale OnComponentBeginOverlap(beam) OtherActor)) (Math|Transform|MakeTransform (.location _returnvalue_2) (.rotation _returnvalue_2) "1.000000,1.000000,1.000000") false false)
    (if (== (stale OnComponentBeginOverlap(beam) OtherActor) _returnvalue)
      (Pawn|SetControlRotation (Game|GetPlayerController 0) (Transformation|GetActorRotation _returnvalue))
      (Variables|/Script/Engine.MovementComponent|SetVelocity (Variables|/Script/Engine.Character|GetCharacterMovement _returnvalue) "0, 0, 0"))))

(fn ConstructionScript
  (Transformation|SetRelativeTransform (Variables|Default|GetArrow) (Variables|Default|GetTeleport%20Location) false false))